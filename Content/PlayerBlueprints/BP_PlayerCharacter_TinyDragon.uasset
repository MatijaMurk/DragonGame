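; Player character Blueprint for a tiny dragon that gets a random look each time it spawns.
; On BeginPlay it calls the parent, then creates a dynamic material instance on the mesh's first slot from a randomly picked entry among five in MaterialArray.
; Tick and the construction script only call the parent, and the overlap event is disabled, so any other behavior comes from the parent class.
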(event EventBeginPlay
  (|CallParentFunction)
  ;[1 0.7211 0.5154] Set random material on spawn
  (Rendering|Material|CreateDynamicMaterialInstance (Variables|Character|GetMesh) 0 (Utilities|Array|Get(acopy) (Variables|Default|GetMaterialArray) (Math|Random|RandomIntegerinRange 0 4)) "None" :!class /Script/Engine.PrimitiveComponent))

(event Collision|EventActorBeginOverlap
  (params (OtherActor :type Actor%20Object%20Reference))
  (|CallParentFunction OtherActor) ; This node is disabled and will not be called.\nDrag off pins to build functionality.
)

(event EventTick
  (params (DeltaSeconds :type Float%20%28single-precision%29))
  (|CallParentFunction DeltaSeconds))

(fn ConstructionScript
  (|CallParentFunction))