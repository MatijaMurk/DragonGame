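; Base enemy Blueprint that takes damage, shows damage numbers and awards XP to the player on death.
; EnemyStatsComponent holds HP and the XP reward, which is copied from the actor's XPtoGive on BeginPlay.
; AnyDamage spawns a DamageInd widget at the enemy's projected screen position with random offset, then calls ChangeHealth.
; At zero HP, ChangeHealth grants XP to the Player reference set by NewPlayer and destroys the actor.
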(event EventBeginPlay
  (Variables|/Game/SimpleEnemy/EnemyStatsComponent.EnemyStatsComponent_C|SetXPtoGive (Variables|Default|GetEnemyStatsComponent) (Variables|Default|GetXPtoGive)))

(event Game|Damage|EventAnyDamage
  (params (Damage :type Float%20%28single-precision%29) (DamageType :type Damage%20Type%20Object%20Reference) (InstigatedBy :type Controller%20Object%20Reference) (DamageCauser :type Actor%20Object%20Reference))
  (bind _returnvalue (UserInterface|CreateWidget "/Game/UI/DamageInd.DamageInd_C" 0 Damage))
  (UserInterface|Viewport|AddtoViewport _returnvalue 0)
  (Class|UserWidget|SetPositioninViewport _returnvalue (+ (.ScreenPosition (Class|WidgetLayoutLibrary|ProjectWorldLocationtoWidgetPosition (Game|GetPlayerController 0) (Transformation|GetActorLocation self) true)) (Math|Random|RandomFloatinRange -75.0 75.0)) false)
  (CallFunction|ChangeHealth (Math|Float|Truncate Damage)))

(event EventNewPlayer
  (bind _asbp_player_character_master (Utilities|Casting|CastToBP_PlayerCharacter_Master (Game|GetPlayerCharacter 0)))
  (Variables|Default|SetPlayer _asbp_player_character_master))

(fn ConstructionScript)

(fn ChangeHealth
  (params (DamageTaken :type Integer))
  (bind _enemystatscomponent (Variables|Default|GetEnemyStatsComponent))
  (bind _output_get (Variables|/Game/SimpleEnemy/EnemyStatsComponent.EnemyStatsComponent_C|SetCurrentHP _enemystatscomponent (- (Variables|/Game/SimpleEnemy/EnemyStatsComponent.EnemyStatsComponent_C|GetCurrentHP _enemystatscomponent) DamageTaken)))
  (if (<= _output_get 0)
    (Default|ChangeXP (Variables|Default|GetPlayer) (Variables|/Game/SimpleEnemy/EnemyStatsComponent.EnemyStatsComponent_C|GetXPtoGive (Variables|Default|GetEnemyStatsComponent)))
    (Actor|DestroyActor)))